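; WorldItem is a clickable item in the game world that the player can pick up.
; Its static mesh comes from its Item data, set in the construction script on the authority and at BeginPlay on remote clients.
; Clicking it casts player character 0 to MMOPlayerCharacter and passes the item to PickUpItem, leaving the pickup logic to the character.
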(event `self.ReceiveActorOnClicked`
  (`/Game/MMO/Blueprints/MMOPlayerCharacter.PickUpItem` (cast `/Game/MMO/Blueprints/MMOPlayerCharacter` (`GameplayStatics.GetPlayerCharacter` 0) :!pure true) self))

(event `self.ReceiveBeginPlay`
  (`/Engine/EditorBlueprintResources/ActorMacros.Switch Has Authority`
    (:`Remote`
      (`StaticMeshComponent.SetStaticMesh` (`ItemData.Mesh` (`self.Item`))))))

(event `self.ReceiveActorBeginOverlap`
  (params (OtherActor :type "Actor Object Reference")))

(event `self.ReceiveTick`
  (params (DeltaSeconds :type "Float (single-precision)")))

(fn `UserConstructionScript`
  (`/Engine/EditorBlueprintResources/ActorMacros.Switch Has Authority`
    (:`Authority`
      (`StaticMeshComponent.SetStaticMesh` (`ItemData.Mesh` (`self.Item`))))))