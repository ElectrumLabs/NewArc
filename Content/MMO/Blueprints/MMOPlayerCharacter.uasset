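; Player character for the MMO, handling targeting, death and respawn, out-of-combat regen, chat commands, group UI and hotbar.
; Server-side events manage slot-based stacking inventory, looting, item pickup/drop and quests, then push updates to client HUD and windows.
; Inventory changes recount collect-quest progress, while NPC overlaps toggle local quest signs.
; The client streams yaw packed into one byte on a timer; disconnect sends a database save request and kicks group membership.
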(event `ChatWhoResponse`
  (params (NumberOfPlayers :type Integer))
  ;[0.2174 0.6535 1] Chat /who command
  (`/Game/MMO/Blueprints/Chat/ChatWidget.AddToMainLog` (`/Game/MMO/Blueprints/MacroLibrary.Chat`) (`|FormatText` "Characters online: {0}" (`KismetTextLibrary.Conv_IntToText` NumberOfPlayers)) (struct :`R` 1.0 :`G` 1.0 :`B` 1.0 :`A` 1.0)))

(event `ChatCommandUnstuck`
  ;[0.2174 0.6535 1] Chat /unstuck command
  (`self.K2_SetActorTransform` (`/Game/MMO/Blueprints/GameModes/MMOGame.RespawnPoint` (cast `/Game/MMO/Blueprints/GameModes/MMOGame` (`GameplayStatics.GetGameMode`) :!pure true))))

(event `self.Assign Target`
  (params (TargetToAssign :type "/Game/MMO/Blueprints/MMOCharacter Object Reference"))
  (bind _mmoinstance (`/Game/MMO/Blueprints/MacroLibrary.MMOInstance`))
  ;[0.6761 0.4477 1] Assign target
  (if (!= TargetToAssign (`self.CurrentTarget`))
    (`self.ClearTarget`)
    (set `self.CurrentTarget` TargetToAssign)
    (`self.Set Target Highlights`)
    ;[0.6761 0.4477 1] Show UI panel with target's stats
    (`Widget.SetVisibility` (`/Game/MMO/Blueprints/UserInterface/GameHUD.[TargetPanel]` (`/Game/MMO/Blueprints/GameModes/MMOInstance.GameHUDWidget` _mmoinstance)) "SelfHitTestInvisible")
    (set `/Game/MMO/Blueprints/UserInterface/TargetText.Character` (`self.CurrentTarget`) (`/Game/MMO/Blueprints/GameModes/MMOInstance.TargetText` _mmoinstance))))

(event `ChatCommandWho`
  ;[0.2174 0.6535 1] Chat /who command
  (bind _returnvalue (`GameModeBase.GetNumPlayers` (`GameplayStatics.GetGameMode`)))
  (`self.ChatWhoResponse` _returnvalue))

(event `TurnInQuest`
  (params (Quest :type "Quest Object Reference") (RewardIndex :type Integer :default 0))
  ;[0.09093 1 0.3993] Turn in quest
  (bind (_true _index) (`self.HasQuest` Quest))
  (if _true
    (`KismetArrayLibrary.Array_Add` (`self.CompletedQuests`) Quest)
    (bind _success (`self.AddToSuitableInventorySlot` (`|GetArrayItem` (`Quest.Rewards` Quest) RewardIndex) 1))
    (if _success
      (`KismetArrayLibrary.Array_Remove` (`self.AcceptedQuests`) _index)
      (`self.UpdateAcceptedCompletedQuests` (`self.AcceptedQuests`) (`self.CompletedQuests`)))))

(event `self.OnDeathServer`
  ;[0.94 0.4685 0.3196] Server: OnDeath
  (`self.StopAttacking`)
  (`KismetArrayLibrary.Array_Clear` (`self.InCombatWith`))
  ;[0.4707 1 0.465] Player respawn (automatically)
  (`KismetSystemLibrary.K2_SetTimerDelegate` (delegate `Respawn Server`) (`self.RespawnTime`)))

(event `Respawn Server`
  ;[0.4707 1 0.465] Player respawn (automatically)
  (`self.K2_SetActorTransform` (`/Game/MMO/Blueprints/GameModes/MMOGame.RespawnPoint` (cast `/Game/MMO/Blueprints/GameModes/MMOGame` (`GameplayStatics.GetGameMode`) :!pure true)))
  (set `self.HP` (`self.MaxHP`))
  (`self.SetActorHiddenInGame` false)
  (`self.RespawnClient`)
  (`KismetSystemLibrary.K2_ClearTimer` self "HideBody"))

(event `self.K2_OnEndViewTarget`
  (params (PC :type "PlayerController Object Reference"))
  ;[1 0.5989 0.6276] Server: On disconnect, store character transform in the db
  (`/Engine/EditorBlueprintResources/ActorMacros.Switch Has Authority`
    (:`Authority`
      (`/Game/MMO/Blueprints/MMOPlayerState.SendRequest` (cast `/Game/MMO/Blueprints/MMOPlayerState` (`Controller.PlayerState` PC) :!pure true) "NewEnumerator4"))))

(event `AcceptQuest`
  (params (Quest :type "Quest Object Reference"))
  ;[0.09093 1 0.3993] Accept quest
  (bind _taskprogress (`self.MakeEmptyTaskProgress` Quest))
  (`KismetArrayLibrary.Array_Add` (`self.AcceptedQuests`) (make `/Game/MMO/Quests/AcceptedQuest` Quest _taskprogress))
  (`self.UpdateCollectTaskProgress`) ; in case the required items were already in the inventory
  (`self.UpdateAcceptedCompletedQuests` (`self.AcceptedQuests`) (`self.CompletedQuests`)))

(event `self.ReceiveActorBeginOverlap`
  (params (OtherActor :type "Actor Object Reference"))
  ;[0.6761 0.4477 1] When our character is close to an NPC, spawn quest sign if it's a quest start/end NPC
  (if (and (not (`KismetSystemLibrary.IsDedicatedServer`)) (`self.IsLocallyControlled`))
    (`/Game/MMO/AI/NPC.RefreshSign` (cast `/Game/MMO/AI/NPC` OtherActor :!pure true))))

(event `RespawnClient`
  ;[1 1 1] Client: respawn: unlock movement, clear target and hostility
  (set `self.MovementLocked` false)
  (`self.ClearTarget`)
  (bind _outactors (`GameplayStatics.GetAllActorsOfClass` "/Game/MMO/AI/AICharacter.AICharacter_C"))
  (for _array_element _outactors
    (bind _asaicharacter (cast `/Game/MMO/AI/AICharacter` _array_element))
    (set `/Game/MMO/Blueprints/MMOCharacter.Hostility` "NewEnumerator1" _asaicharacter)))

(event `self.ReceiveEndPlay`
  (params (EndPlayReason :type "EEndPlayReason Enum" :default "Destroyed"))
  (bind _namewidget (`self.NameWidget`))
  (bind _serverchatconnect (`/Game/MMO/Blueprints/GameModes/MMOGame.ServerChatConnect` (cast `/Game/MMO/Blueprints/GameModes/MMOGame` (`GameplayStatics.GetGameMode`) :!pure true)))
  ;[1 1 1] On disconnect - kick player from their group
  (`/Engine/EditorBlueprintResources/ActorMacros.Switch Has Authority`
    (:`Authority`
      (`/Engine/EditorBlueprintResources/StandardMacros.IsValid` _serverchatconnect
        (:`Is Valid`
          (`ChatConnect.GroupKick` _serverchatconnect (`KismetTextLibrary.Conv_TextToString` (`self.Name`))))))
    (:`Remote`
      (`/Engine/EditorBlueprintResources/StandardMacros.IsValid` _namewidget
        (:`Is Valid`
          (`Widget.RemoveFromParent` _namewidget))))))

(event `UpdateAcceptedCompletedQuests`
  (params (AcceptedQuests :type "Array of /Game/MMO/Quests/AcceptedQuest Structure") (CompletedQuests :type "Array of Quest Object Reference"))
  ;[0.09093 1 0.3993] Update accepted quests
  (bind _output_get (set `self.AcceptedQuests` AcceptedQuests))
  (set `self.CompletedQuests` CompletedQuests)
  (`/Game/MMO/Blueprints/UserInterface/GameHUD.UpdateTrackedQuests` (`/Game/MMO/Blueprints/GameModes/MMOInstance.GameHUDWidget` (`/Game/MMO/Blueprints/MacroLibrary.MMOInstance`)) _output_get)
  (`self.RefreshNPCsigns`))

(event `self.ReceiveActorEndOverlap`
  (params (OtherActor :type "Actor Object Reference"))
  ;[0.6761 0.4477 1] When a quest NPC becomes too far away, hide its quest sign
  (if (and (not (`KismetSystemLibrary.IsDedicatedServer`)) (`self.IsLocallyControlled`))
    (`SceneComponent.SetHiddenInGame` (`/Game/MMO/AI/NPC.QuestEndSign` (cast `/Game/MMO/AI/NPC` OtherActor :!pure true)) true false)
    (`SceneComponent.SetHiddenInGame` (`/Game/MMO/AI/NPC.QuestStartSign` (cast `/Game/MMO/AI/NPC` OtherActor :!pure true)) true false)))

(event `RefreshNPCsigns`
  ;[0.6761 0.4477 1] Refresh NPC signs
  (for _array_element (`PrimitiveComponent.GetOverlappingActors` "/Game/MMO/AI/NPC.NPC_C")
    (`/Game/MMO/AI/NPC.RefreshSign` (cast `/Game/MMO/AI/NPC` _array_element :!pure true))))

(event `ReceiveOwnRotation`
  (params (Rotation :type "Rotator Structure"))
  (`self.K2_SetActorRotation` Rotation))

(event `self.ReceiveBeginPlay`
  (bind _returnvalue (`GameplayStatics.GetPlayerCharacter` 0))
  ;[0.3767 1 0.37] Begin play: start health regeneration
  (`parent.ReceiveBeginPlay`)
  (`/Engine/EditorBlueprintResources/ActorMacros.Switch Has Authority`
    (:`Authority`
      (`KismetSystemLibrary.K2_SetTimerDelegate` (delegate `TickRegen`) 2.0 true))
    (:`Remote`
      (`|ExecutionSequence`
        (:`then_0`
          ;[1 1 1] Create name widget
          (bind _returnvalue_2 (`|CreateWidget` "/Game/MMO/Blueprints/UserInterface/TargetText.TargetText_C" null self))
          (bind _output_get (set `self.NameWidget` _returnvalue_2))
          (`UserWidget.AddToViewport` _output_get 0))
        (:`then_1`
          ;[1 1 1] check if the new character is in our group (to update their hp bar)
          (`/Engine/EditorBlueprintResources/StandardMacros.IsValid` _returnvalue
            (:`Is Valid`
              (for _array_element (`/Game/MMO/Blueprints/MMOPlayerCharacter.GroupMembers` (cast `/Game/MMO/Blueprints/MMOPlayerCharacter` _returnvalue :!pure true))
                (if (`KismetStringLibrary.EqualEqual_StrStr` (`.Name_5_63085C0A409FEEC058DB5FAA79FC0397` (break `/Game/MMO/Blueprints/Groups/CrossServerPlayer` _array_element)) (`KismetTextLibrary.Conv_TextToString` (`self.Name`)))
                  (`/Game/MMO/Blueprints/UserInterface/GameHUD.UpdateGroupMember` (`/Game/MMO/Blueprints/GameModes/MMOInstance.GameHUDWidget` (`/Game/MMO/Blueprints/MacroLibrary.MMOInstance`)) self))))))))))

(event `ChatLogin`
  (params (Name :type String))
  ;[1 1 1] Client: Login to chat as <charactername> (after entered world)
  (`ChatConnect.Login` (`/Game/MMO/Blueprints/Chat/ChatWidget.ChatConnect` (`/Game/MMO/Blueprints/MacroLibrary.Chat`)) Name)
  (`KismetSystemLibrary.Delay` 1.0)
  (`MyGameInstance.EndLoadingScreen` (`/Game/MMO/Blueprints/MacroLibrary.MMOInstance`)))

(event `TickRegen`
  ;[0.3767 1 0.37] Begin play: start health regeneration
  (if (and (`/Game/MMO/Blueprints/ObjectMacroLibrary.is Empty` (`self.InCombatWith`)) (> (`self.HP`) 0))
    (set `self.HP` (`KismetMathLibrary.Clamp` (+ (`self.HP`) 10) 0 (`self.MaxHP`)))))

(event `self.OnSlainSomethingClient`
  (params (`Attack Target` :type "/Game/MMO/Blueprints/MMOCharacter Object Reference"))
  ;[1 1 1] Log when this player character has slain something
  (`/Game/MMO/Blueprints/Chat/ChatWidget.Log Slain` (`/Game/MMO/Blueprints/MacroLibrary.Chat`) self `Attack Target`))

(event `self.K2_OnBecomeViewTarget`
  (params (PC :type "PlayerController Object Reference"))
  ;[1 1 1] OnBecomeViewTarget Client: send character rotation to server
  (`/Engine/EditorBlueprintResources/ActorMacros.Switch Has Authority`
    (:`Remote`
      (if (`self.IsLocallyControlled`)
        (`KismetSystemLibrary.Delay` 2.0)
        (`KismetSystemLibrary.K2_SetTimerDelegate` (delegate `ClientSendRotation`) 0.05 true)))))

(event `ClientSendRotation`
  ;[1 1 1] OnBecomeViewTarget Client: send character rotation to server
  (`self.ServerSetRotation` (`KismetMathLibrary.Conv_IntToByte` (`KismetMathLibrary.FFloor` (* (/ (+ (.yaw (`self.K2_GetActorRotation`)) 180.0) 360.0) 255.0)))))

(event `TryToLoot`
  (params (TargetToLoot :type "/Game/MMO/Blueprints/MMOCharacter Object Reference"))
  ;[0.851 0.3052 0] Opening loot container
  (if (`KismetArrayLibrary.Array_Contains` (`/Game/MMO/Blueprints/MMOCharacter.LootRights` TargetToLoot) self)
    (set `self.CurrentOpenLoot` TargetToLoot)
    (`self.OpenLootContainer` (`/Game/MMO/Blueprints/MMOCharacter.Name` TargetToLoot) (`/Game/MMO/Blueprints/MMOCharacter.Inventory` TargetToLoot))))

(event `UpdateInventory`
  (params (Items :type "Array of /Game/MMO/Blueprints/Inventory/InventoryItem Structure"))
  (bind _inventory (`/Game/MMO/Blueprints/UserInterface/FullUI.Inventory` (`/Game/MMO/Blueprints/GameModes/MMOInstance.FullUIWidget` (`/Game/MMO/Blueprints/MacroLibrary.MMOInstance`))))
  ;[0.851 0.2537 0] Client: Update Inventory
  (set `self.Inventory` Items)
  (`/Engine/EditorBlueprintResources/StandardMacros.IsValid` _inventory
    (:`Is Valid`
      (`/Game/MMO/Blueprints/Inventory/Inventory.LoadItems` _inventory Items))))

(event `ServerSetRotation`
  (params (Value :type Byte))
  ;[1 1 1] OnBecomeViewTarget Client: send character rotation to server
  (`self.K2_SetActorRotation` (`KismetMathLibrary.MakeRotator` 0.0 0.0 (`KismetMathLibrary.Lerp` -180.0 180.0 (/ (`KismetMathLibrary.Conv_ByteToDouble` Value) 255.0)))))

(event `OpenLootContainer`
  (params (Name :type Text) (Items :type "Array of /Game/MMO/Blueprints/Inventory/InventoryItem Structure"))
  (bind _container (`/Game/MMO/Blueprints/UserInterface/FullUI.Container` (`/Game/MMO/Blueprints/GameModes/MMOInstance.FullUIWidget` (`/Game/MMO/Blueprints/MacroLibrary.MMOInstance`))))
  ;[0.851 0.3052 0] Opening loot container
  (`/Game/MMO/Blueprints/Inventory/Inventory.LoadItems` _container Items)
  (`/Game/MMO/Blueprints/Inventory/Inventory.ChangeWindowTitle` _container Name)
  (`Widget.SetVisibility` (`/Game/MMO/Blueprints/Inventory/Inventory.DraggableWindow` _container) "SelfHitTestInvisible"))

(event `UpdateGroupMembers`
  (params (Members :type "Array of /Game/MMO/Blueprints/Groups/CrossServerPlayer Structure"))
  ;[0.2474 0.755 0.2506] Update Group Members
  (bind _output_get (set `self.GroupMembers` Members))
  (`/Game/MMO/Blueprints/UserInterface/GameHUD.DisplayGroupMembers` (`/Game/MMO/Blueprints/GameModes/MMOInstance.GameHUDWidget` (`/Game/MMO/Blueprints/MacroLibrary.MMOInstance`)) _output_get))

(event `UpdateHotbar`
  (params (`New Hotbar` :type "Array of HotbarObject Object Reference"))
  ;[0.996 1 0.3327] Update Hotbar
  (bind _output_get (set `self.Hotbar` `New Hotbar`))
  (`/Game/MMO/Blueprints/UserInterface/GameHUD.LoadHotbar` (`/Game/MMO/Blueprints/GameModes/MMOInstance.GameHUDWidget` (`/Game/MMO/Blueprints/MacroLibrary.MMOInstance`)) _output_get))

(event `LootItem`
  (params (Slot :type Integer))
  (bind _currentopenloot (`self.CurrentOpenLoot`))
  (bind _inventory (`/Game/MMO/Blueprints/MMOCharacter.Inventory` _currentopenloot))
  ;[0.851 0.3052 0] Looting
  (bind (_inventoryitem _hasitem _arrayindex) (`self.FindInventoryStackBySlotIndex` (`self.CurrentOpenLoot`) Slot))
  (if _hasitem
    (bind (_item _amount) (break `/Game/MMO/Blueprints/Inventory/InventoryItem` _inventoryitem))
    (bind _success (`self.AddToSuitableInventorySlot` _item _amount))
    (if _success
      (`KismetArrayLibrary.Array_Remove` _inventory _arrayindex)
      (`self.OpenLootContainer` (`/Game/MMO/Blueprints/MMOCharacter.Name` _currentopenloot) _inventory) ; refresh container
    )))

(event `ReceiveLoot`
  (params (Item :type "ItemData Object Reference"))
  ;[0.851 0.3052 0] Client: ReceiveLoot
  (`/Game/MMO/Blueprints/Chat/ChatWidget.Log Receive Loot` (`/Game/MMO/Blueprints/MacroLibrary.Chat`) Item)
  (`GameplayStatics.PlaySound2D` (`ItemData.PickSound` Item)))

(event `MoveInventoryStack`
  (params (NewSlot :type Integer) (OldSlot :type Integer))
  ;[0.851 0.2537 0] Server:Move/Destroy inventory stack
  (`self.MoveInventoryStackFunc` NewSlot OldSlot)
  (`self.UpdateInventory` (`self.Inventory`) :!label _label))

(event `DestroyInventoryStack`
  (params (Slot :type Integer))
  ;[0.851 0.2537 0] Server:Move/Destroy inventory stack
  (bind (_inventoryitem _hasitem _arrayindex) (`self.FindInventoryStackBySlotIndex` Slot))
  (`KismetArrayLibrary.Array_Remove` (`self.Inventory`) _arrayindex)
  (`self.UpdateCollectTaskProgress`)
  (goto _label))

(event `PickUpItem`
  (params (LootableItem :type "/Game/MMO/Blueprints/WorldItem Object Reference"))
  ;[0.851 0.3979 0.1447] Server: Pick up item
  (`/Engine/EditorBlueprintResources/StandardMacros.IsValid` LootableItem
    (:`Is Valid`
      (bind _success (`self.AddToSuitableInventorySlot` (`/Game/MMO/Blueprints/WorldItem.Item` LootableItem) 1))
      (if _success
        (`self.K2_DestroyActor` LootableItem)))))

(event `Dropitem`
  (params (Slot :type Integer))
  (bind _inventory (`self.Inventory`))
  (bind _returnvalue (`KismetMathLibrary.MakeVector` (+ (.x (.location (`self.GetTransform`))) 100.0) (.y (.location (`self.GetTransform`))) (+ (.z (.location (`self.GetTransform`))) 90.0)))
  ;[0.851 0.3979 0.1447] Server: Drop item
  (bind _inventoryitem (`self.FindInventoryStackBySlotIndex` Slot))
  (bind (_item _amount) (break `/Game/MMO/Blueprints/Inventory/InventoryItem` _inventoryitem))
  (if (and (`ItemData.isStackable` _item) (> _amount 1))
    (bind (_item_2 _amount_2 _slotnumber) (break `/Game/MMO/Blueprints/Inventory/InventoryItem` _inventoryitem))
    (`KismetArrayLibrary.Array_Set` _inventory 0 (make `/Game/MMO/Blueprints/Inventory/InventoryItem` _item_2 (- _amount_2 1) _slotnumber))
    (`self.UpdateInventory` _inventory)
    (`self.UpdateCollectTaskProgress`)
    (else
      (`self.DestroyInventoryStack` Slot)))
  (bind _outhit (`KismetSystemLibrary.LineTraceSingleForObjects` _returnvalue (- _returnvalue (0.0 0.0 500.0)) (`|MakeArray` "ObjectTypeQuery1" "ObjectTypeQuery7" :!type "EObjectTypeQuery Enum")))
  (`|SpawnActorFromClass` "/Game/MMO/Blueprints/WorldItem.WorldItem_C" (`KismetMathLibrary.Conv_VectorToTransform` (`.Location` (`GameplayStatics.BreakHitResult` _outhit))) "AdjustIfPossibleButAlwaysSpawn" "OverrideRootScale" null _item))

(fn `AddToSuitableInventorySlot`
  (params (Item :type "ItemData Object Reference") (Amount :type Integer))
  (returns (Success :type Boolean))
  (if (`ItemData.isStackable` Item)
    ;[1 1 1] for stackable items, first try to find a suitable existing stack
    (for (_array_element _array_index) (`self.Inventory`)
      (bind (_item _amount _slotnumber) (break `/Game/MMO/Blueprints/Inventory/InventoryItem` _array_element))
      (bind _returnvalue (+ _amount Amount))
      (if (and (== _item Item) (<= _returnvalue 20))
        (`KismetArrayLibrary.Array_Set` (`self.Inventory`) _array_index (make `/Game/MMO/Blueprints/Inventory/InventoryItem` _item _returnvalue _slotnumber))
        (`|ExecutionSequence`
          (:`then_0`
            (break))
          (:`then_1`
            (`self.ReceiveLoot` Item :!label _label)
            (`self.UpdateInventory` (`self.Inventory`)) ; refresh inventory
            ;[0.09093 1 0.3993] Update "collect" quests
            (`self.UpdateCollectTaskProgress`)
            (return true))))))
  (bind (_output _exists) (`self.GetEmptyInventorySlot`))
  (if _exists
    (`KismetArrayLibrary.Array_Add` (`self.Inventory`) (make `/Game/MMO/Blueprints/Inventory/InventoryItem` Item Amount _output))
    (goto _label)
    (else
      (return false))))

(fn `HasItem`
  (params (Item :type "ItemData Object Reference"))
  (returns (Count :type Integer))
  (locals (Output :type Integer))
  (for _array_element (`self.Inventory`)
    (bind (_item _amount) (break `/Game/MMO/Blueprints/Inventory/InventoryItem` _array_element))
    (if (== _item Item)
      (set `local.Output` (+ (`local.Output`) _amount))))
  (return (`local.Output`)))

(fn `HasQuest`
  (params (Quest :type "Quest Object Reference"))
  (returns (True :type Boolean) (Index :type Integer))
  (locals (Output :type Boolean) (OutputIndex :type Integer :default -1))
  (for (_array_element _array_index) (`self.AcceptedQuests`)
    (if (== Quest (`.Quest_6_0AA7FD564A172E5E02319C9605112C3A` (break `/Game/MMO/Quests/AcceptedQuest` _array_element)))
      (set `local.Output` true)
      (set `local.OutputIndex` _array_index)
      (break)))
  (return (`local.Output`) (`local.OutputIndex`)))

(fn `MakeEmptyTaskProgress`
  (params (Quest :type "Quest Object Reference"))
  (returns (TaskProgress :type "Array of Integer"))
  (locals (Output :type "Array of Integer"))
  (for _ (`Quest.BringTasks` Quest)
    (`KismetArrayLibrary.Array_Add` (`local.Output`) :!label _label))
  (for _ (`Quest.KillTasks` Quest)
    (goto _label))
  (return (`local.Output`)))

(fn `MoveInventoryStackFunc`
  (params (NewSlotIndex :type Integer) (OldSlotIndex :type Integer))
  (locals (NewSlot :type Integer) (OldSlot :type Integer) (AmountToMove :type Integer) (ItemToMove :type "ItemData Object Reference") (OriginArrayIndex :type Integer) (TargetArrayIndex :type Integer) (StackMaximum :type Integer) (AmountInTargetSlot :type Integer) (ItemInTargetSlot :type "ItemData Object Reference"))
  (bind _inventory (`self.Inventory`))
  (bind _inventory_2 (`self.Inventory`))
  (bind _stackmaximum (`local.StackMaximum`))
  (bind _originarrayindex (`local.OriginArrayIndex`))
  (bind _itemintargetslot (`local.ItemInTargetSlot`))
  (bind _returnvalue (+ (`local.AmountInTargetSlot`) (`local.AmountToMove`)))
  (bind _returnvalue_2 (- _returnvalue _stackmaximum))
  (set `local.StackMaximum` 20)
  (set `local.NewSlot` NewSlotIndex)
  (set `local.OldSlot` OldSlotIndex)
  (bind (_inventoryitem _hasitem _arrayindex) (`self.FindInventoryStackBySlotIndex` (`local.OldSlot`)))
  (set `local.OriginArrayIndex` _arrayindex)
  (bind (_item _amount) (break `/Game/MMO/Blueprints/Inventory/InventoryItem` _inventoryitem))
  (set `local.ItemToMove` _item)
  (set `local.AmountToMove` _amount)
  (bind (_inventoryitem_2 _hasitem_2 _arrayindex_2) (`self.FindInventoryStackBySlotIndex` (`local.NewSlot`)))
  (set `local.TargetArrayIndex` _arrayindex_2)
  (bind (_item_2 _amount_2) (break `/Game/MMO/Blueprints/Inventory/InventoryItem` _inventoryitem_2))
  (set `local.ItemInTargetSlot` _item_2)
  (set `local.AmountInTargetSlot` _amount_2)
  (if _hasitem_2
    (if (and (`ItemData.isStackable` _itemintargetslot) (== _itemintargetslot (`local.ItemToMove`)))
      ;[1 1 1] Adding to an existing stack
      (`KismetArrayLibrary.Array_Set` (`self.Inventory`) (`local.TargetArrayIndex`) (make `/Game/MMO/Blueprints/Inventory/InventoryItem` (`local.ItemToMove`) (`KismetMathLibrary.Min` _returnvalue _stackmaximum) (`local.NewSlot`)))
      (if (<= _returnvalue_2 0)
        (`KismetArrayLibrary.Array_Remove` _inventory _originarrayindex)
        (else
          (`KismetArrayLibrary.Array_Set` _inventory _originarrayindex (make `/Game/MMO/Blueprints/Inventory/InventoryItem` (`local.ItemToMove`) _returnvalue_2 (`local.OldSlot`)))))
      (else
        ;[1 1 1] Switching different or unstackable items
        (`KismetArrayLibrary.Array_Set` _inventory_2 (`local.TargetArrayIndex`) (make `/Game/MMO/Blueprints/Inventory/InventoryItem` (`local.ItemToMove`) (`local.AmountToMove`) (`local.NewSlot`)))
        (`KismetArrayLibrary.Array_Set` _inventory_2 (`local.OriginArrayIndex`) (make `/Game/MMO/Blueprints/Inventory/InventoryItem` (`local.ItemInTargetSlot`) (`local.AmountInTargetSlot`) (`local.OldSlot`)))))
    (else
      ;[1 1 1] Movement to an empty slot
      (`KismetArrayLibrary.Array_Set` (`self.Inventory`) (`local.OriginArrayIndex`) (make `/Game/MMO/Blueprints/Inventory/InventoryItem` (`local.ItemToMove`) (`local.AmountToMove`) (`local.NewSlot`))))))

(fn `UpdateCollectTaskProgress`
  (locals (Temp :type "Array of Integer"))
  (for (_array_element _array_index) (`self.AcceptedQuests`)
    (bind (_quest _taskprogress) (break `/Game/MMO/Quests/AcceptedQuest` _array_element))
    (set `local.Temp` _taskprogress)
    (for (_array_element_2 _array_index_2) (`Quest.BringTasks` _quest)
      (bind (_itemtobring _amounttobring) (break `QuestTaskBring` _array_element_2))
      (bind _count (`self.HasItem` _itemtobring))
      (`KismetArrayLibrary.Array_Set` (`local.Temp`) _array_index_2 (`KismetMathLibrary.Clamp` _count 0 _amounttobring)))
    (`KismetArrayLibrary.Array_Set` (`self.AcceptedQuests`) _array_index (make `/Game/MMO/Quests/AcceptedQuest` _quest (`local.Temp`))))
  ;[1 1 1] send the update to the client
  (`self.UpdateAcceptedCompletedQuests` (`self.AcceptedQuests`) (`self.CompletedQuests`)))

(fn `UserConstructionScript`
  (`parent.UserConstructionScript`))